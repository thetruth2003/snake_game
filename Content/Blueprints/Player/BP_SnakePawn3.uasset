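; Snake pawn variant that lets a player steer in four directions and jump, with SetNextDirection and Jump defined outside this graph.
; On BeginPlay it adds the IMC_Player3 Enhanced Input mapping context to its controller, though the handled input actions carry P2 names.
; Each tick, UpdateHeadRotation quaternion-slerps the Head's relative rotation toward ForwardRotation, scaled by delta time, for smooth turning.
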(event Input|EnhancedActionEvents|EnhancedInputActionMoveUp_P2
  (params (ActionValue :type Boolean) (ElapsedSeconds :type Float%20%28double-precision%29) (TriggeredSeconds :type Float%20%28double-precision%29) (InputAction :type Input%20Action%20Object%20Reference :default "/Game/Input/Actions/MoveUp_P2.MoveUp_P2"))
  (Class|SnakePawn|SetNextDirection "Up"))

(event Input|EnhancedActionEvents|EnhancedInputActionMoveRight_P2
  (params (ActionValue :type Boolean) (ElapsedSeconds :type Float%20%28double-precision%29) (TriggeredSeconds :type Float%20%28double-precision%29) (InputAction :type Input%20Action%20Object%20Reference :default "/Game/Input/Actions/MoveRight_P2.MoveRight_P2"))
  (Class|SnakePawn|SetNextDirection "Right"))

(event Input|EnhancedActionEvents|EnhancedInputActionMoveDown_P2
  (params (ActionValue :type Boolean) (ElapsedSeconds :type Float%20%28double-precision%29) (TriggeredSeconds :type Float%20%28double-precision%29) (InputAction :type Input%20Action%20Object%20Reference :default "/Game/Input/Actions/MoveDown_P2.MoveDown_P2"))
  (Class|SnakePawn|SetNextDirection "Down"))

(event Input|EnhancedActionEvents|EnhancedInputActionJump_P2
  (params (ActionValue :type Boolean) (ElapsedSeconds :type Float%20%28double-precision%29) (TriggeredSeconds :type Float%20%28double-precision%29) (InputAction :type Input%20Action%20Object%20Reference :default "/Game/Input/Actions/Jump_P2.Jump_P2"))
  (Class|SnakePawn|Jump))

(event Input|EnhancedActionEvents|EnhancedInputActionMoveLeft__P2
  (params (ActionValue :type Boolean) (ElapsedSeconds :type Float%20%28double-precision%29) (TriggeredSeconds :type Float%20%28double-precision%29) (InputAction :type Input%20Action%20Object%20Reference :default "/Game/Input/Actions/MoveLeft__P2.MoveLeft__P2"))
  (Class|SnakePawn|SetNextDirection "Left"))

(event EventBeginPlay
  (bind _asplayer_controller (Utilities|Casting|CastToPlayerController (Pawn|GetController)))
  (Input|AddMappingContext (PlayerController|LocalPlayerSubsystems|GetEnhancedInputLocalPlayerSubsystem _asplayer_controller) "/Game/Input/IMC_Player3.IMC_Player3" 0 "(bIgnoreAllPressedKeysUntilRelease=True,bForceImmediately=False,bNotifyUserSettings=False)"))

(event Collision|EventActorBeginOverlap
  (params (OtherActor :type Actor%20Object%20Reference)))

(event EventTick
  (params (DeltaSeconds :type Float%20%28single-precision%29))
  (CallFunction|UpdateHeadRotation DeltaSeconds))

(fn ConstructionScript)

(fn UpdateHeadRotation
  (params (DeltaTime :type Float%20%28double-precision%29))
  (Transformation|SetRelativeRotation (Variables|Default|GetHead) (Class|KismetMathLibrary|QuatRotator (Class|KismetMathLibrary|QuatSlerp (Math|Conversions|ToQuaternion(Rotator) (Variables|/Script/Engine.SceneComponent|GetRelativeRotation (Variables|Default|GetHead))) (Math|Conversions|ToQuaternion(Rotator) (Variables|Default|GetForwardRotation)) (* DeltaTime 2e+01))) false false))