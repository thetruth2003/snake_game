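; BP_SnakePawn2 is a snake pawn, apparently for the second player, that turns movement and jump input into snake actions.
; Enhanced Input actions pass four directions to SetNextDirection or call Jump, neither of which is defined here.
; Tick eases the head toward ForwardRotation with a quaternion slerp scaled by delta time.
; The logic that would add the IMC_Player2 mapping context is unconnected and never runs.
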(event Input|EnhancedActionEvents|EnhancedInputActionIA_MoveUp
  (params (ActionValue :type Boolean) (ElapsedSeconds :type Float%20%28double-precision%29) (TriggeredSeconds :type Float%20%28double-precision%29) (InputAction :type Input%20Action%20Object%20Reference :default "/Game/Input/Actions/IA_MoveUp.IA_MoveUp"))
  (Class|SnakePawn|SetNextDirection "Up"))

(event Input|EnhancedActionEvents|EnhancedInputActionIA_MoveRight
  (params (ActionValue :type Boolean) (ElapsedSeconds :type Float%20%28double-precision%29) (TriggeredSeconds :type Float%20%28double-precision%29) (InputAction :type Input%20Action%20Object%20Reference :default "/Game/Input/Actions/IA_MoveRight.IA_MoveRight"))
  (Class|SnakePawn|SetNextDirection "Right"))

(event Input|EnhancedActionEvents|EnhancedInputActionIA_MoveDown
  (params (ActionValue :type Boolean) (ElapsedSeconds :type Float%20%28double-precision%29) (TriggeredSeconds :type Float%20%28double-precision%29) (InputAction :type Input%20Action%20Object%20Reference :default "/Game/Input/Actions/IA_MoveDown.IA_MoveDown"))
  (Class|SnakePawn|SetNextDirection "Down"))

(event Input|EnhancedActionEvents|EnhancedInputActionIA_MoveLeft
  (params (ActionValue :type Boolean) (ElapsedSeconds :type Float%20%28double-precision%29) (TriggeredSeconds :type Float%20%28double-precision%29) (InputAction :type Input%20Action%20Object%20Reference :default "/Game/Input/Actions/IA_MoveLeft.IA_MoveLeft"))
  (Class|SnakePawn|SetNextDirection "Left"))

(event Input|EnhancedActionEvents|EnhancedInputActionIA_Jump
  (params (ActionValue :type Boolean) (ElapsedSeconds :type Float%20%28double-precision%29) (TriggeredSeconds :type Float%20%28double-precision%29) (InputAction :type Input%20Action%20Object%20Reference :default "/Game/Input/Actions/IA_Jump.IA_Jump"))
  (Class|SnakePawn|Jump))

(event EventBeginPlay)

(event Collision|EventActorBeginOverlap
  (params (OtherActor :type Actor%20Object%20Reference)))

(event EventTick
  (params (DeltaSeconds :type Float%20%28single-precision%29))
  (CallFunction|UpdateHeadRotation DeltaSeconds))

(fn ConstructionScript)

(fn UpdateHeadRotation
  (params (DeltaTime :type Float%20%28double-precision%29))
  (Transformation|SetRelativeRotation (Variables|Default|GetHead) (Class|KismetMathLibrary|QuatRotator (Class|KismetMathLibrary|QuatSlerp (Math|Conversions|ToQuaternion(Rotator) (Variables|/Script/Engine.SceneComponent|GetRelativeRotation (Variables|Default|GetHead))) (Math|Conversions|ToQuaternion(Rotator) (Variables|Default|GetForwardRotation)) (* DeltaTime 2e+01))) false false))